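; Projectile actor that kills BP_Enemy actors on contact and awards a point to its Shooter.
; Tick moves it along world X at ProjSpeed and destroys it once it has lived past a five-second lifetime.
; Cone overlap destroys a hit enemy and the projectile; other overlaps also destroy the projectile, except box components, which it passes through.
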(event OnComponentBeginOverlap(Cone)
  (params (OverlappedComponent :type Primitive%20Component%20Object%20Reference) (OtherActor :type Actor%20Object%20Reference) (OtherComp :type Primitive%20Component%20Object%20Reference) (OtherBodyIndex :type Integer) (bFromSweep :type Boolean) (SweepResult :type Hit%20Result%20Structure%20%28by%20ref%29))
  (bind _shooter (Variables|Default|GetShooter))
  (bind _asbp_enemy (Utilities|Casting|CastToBP_Enemy OtherActor)
    (:then
      (Actor|DestroyActor _asbp_enemy)
      (Variables|/Game/InfiniteMatrix/Blueprints/BP_Player.BP_Player_C|SetScore _shooter (+ (Variables|/Game/InfiniteMatrix/Blueprints/BP_Player.BP_Player_C|GetScore _shooter) 1))
      (Actor|DestroyActor))
    (:CastFailed
      (Utilities|Casting|CastToBoxComponent OtherComp
        (:CastFailed
          (Actor|DestroyActor))))))

(event EventBeginPlay)

(event Collision|EventActorBeginOverlap
  (params (OtherActor :type Actor%20Object%20Reference)))

(event EventTick
  (params (DeltaSeconds :type Float%20%28single-precision%29))
  (Transformation|AddActorWorldOffset (Math|Vector|MakeVector (* DeltaSeconds (Variables|Default|GetProjSpeed)) 0.0 0.0))
  (bind _output_get (Variables|Default|SetTimeAlive (+ (Variables|Default|GetTimeAlive) DeltaSeconds)))
  (if (> _output_get 5.0)
    (Actor|DestroyActor)))

(fn ConstructionScript)